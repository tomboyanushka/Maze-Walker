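; Enemy actor that turns to face and shoots at the first-person character it sees, and dies from projectile hits.
; PawnSensing sightings drive rotation and spawn an enemy projectile, launched by an impulse along the capsule's forward vector.
; A boolean flag with a delay throttles firing.
; Hits from ProjectileActor decrement health, and the enemy is destroyed when it reaches zero.
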(event OnSeePawn(PawnSensing)
  (params (Pawn :type Pawn%20Object%20Reference))
  (bind _asfirst_person_character (Utilities|Casting|CastToFirstPersonCharacter Pawn)
    (:then
      _)
    (:CastFailed
      _))
  (Utilities|FlowControl|Sequence
    (:then_0
      (Transformation|SetActorRotation (Math|Rotator|FindLookatRotation (Transformation|GetActorLocation) (Transformation|GetActorLocation _asfirst_person_character))))
    (:then_1
      (if (Variables|Default|GetSpawnProjectile)
        (bind _returnvalue (Game|SpawnActorfromClass "/Script/Maze.ProjectileActorEnemy" (Transformation|GetWorldTransform (Variables|Default|GetProjectileSpawnLocation)) "Undefined" 0 0))
        (bind _asstatic_mesh_component (Utilities|Casting|CastToStaticMeshComponent (Variables|/Script/Engine.Actor|GetRootComponent _returnvalue)))
        (Physics|AddImpulse _asstatic_mesh_component (* (Math|Vector|GetForwardVector (Variables|Collision|GetCapsuleComponent)) (Variables|Default|GetShootAmount)) "None" false)
        (Variables|Default|SetSpawnProjectile false)
        (Utilities|FlowControl|Delay 2.0)
        (Variables|Default|SetSpawnProjectile true)))))

(event Collision|EventHit
  (params (MyComp :type Primitive%20Component%20Object%20Reference) (Other :type Actor%20Object%20Reference) (OtherComp :type Primitive%20Component%20Object%20Reference) (bSelfMoved :type Boolean) (HitLocation :type Vector :default "0, 0, 0") (HitNormal :type Vector :default "0, 0, 0") (NormalImpulse :type Vector :default "0, 0, 0") (Hit :type Hit%20Result%20Structure%20%28by%20ref%29))
  (bind _enemyhealth (Variables|Default|GetEnemyHealth))
  ;[1 1 1] Death
  (Utilities|Casting|CastToProjectileActor Other)
  (if (stale _bsuccess)
    (Math|Integer|DecrementInt _enemyhealth
      (:%20%20
        (if (== _enemyhealth 0)
          (Actor|DestroyActor))))))

(fn ConstructionScript)